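; BP_Samurai is an actor with a Paper2D sprite of a samurai that slides into position when play begins.
; BeginPlay saves the sprite's relative location as its resting position, then calls the SlideIn event.
; SlideIn plays the SlideInAnim timeline at double speed, using its Alpha to lerp the sprite from SlideStartPos to that saved position.
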(event `self.ReceiveBeginPlay`
  (set `self.SpriteDefaultPos` (`SceneComponent.RelativeLocation` (`self.PaperSprite`)))
  (`self.SlideIn`))

(event `SlideIn`
  (`TimelineComponent.SetPlayRate` (`self.SlideInAnim`) 2.0)
  (bind (_direction _alpha) (`Timeline|SlideInAnim` :!via `PlayFromStart`)
    (:`Update`
      (`SceneComponent.K2_SetRelativeLocationAndRotation` :`self` (`self.PaperSprite`) :`NewLocation` (`KismetMathLibrary.VLerp` (`self.SlideStartPos`) (`self.SpriteDefaultPos`) _alpha)))))

(fn `UserConstructionScript`)